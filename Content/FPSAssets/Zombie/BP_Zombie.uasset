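; Zombie enemy that chases the player, attacks in melee and dies from point damage.
; An AI MoveTo loop retries until it reaches the player, then the attack montage's notify sphere-overlaps at an arrow to apply damage.
; Seeing a pawn raises its walk speed.
; Point damage plays a hit reaction or, when lethal, a death montage, reports the kill to BP_ZombieGameMode and destroys the actor after a delay.
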(event OnSeePawn(PawnSensing)
  (params (Pawn :type Pawn%20Object%20Reference))
  (Variables|/Script/Engine.CharacterMovementComponent|SetMaxWalkSpeed (Variables|Character|GetCharacterMovement) 3.6e+02))

(event Custom|MoveToPlayer
  ;[1 1 1] move logic
  (if (not (Variables|Default|GetIsDead))
    (AI|AIMoveTo self "0, 0, 0" (Game|GetPlayerCharacter 0) 5.0 false
      (:OnSuccess
        (CallFunction|AttackPlayer))
      (:OnFail
        (CallFunction|MovetoPlayer)))))

(event Custom|AttackPlayer
  ;[1 1 1] attack logic
  (bind _asfirst_person_character (Utilities|Casting|CastToFirstPersonCharacter (Game|GetPlayerCharacter 0)))
  (if (not (Variables|/Game/FPSAssets/FirstPersonBP/Blueprints/FirstPersonCharacter.FirstPersonCharacter_C|GetIsDead _asfirst_person_character))
    (Animation|Montage|PlayMontage (Variables|Character|GetMesh) "/Game/FPSAssets/Zombie/Animations/zombie_attack_Montage.zombie_attack_Montage"
      (:OnCompleted
        (CallFunction|MovetoPlayer))
      (:OnNotifyBegin
        (Audio|PlaySoundatLocation "/Game/FPSAssets/Zombie/Sounds/attack.attack" (Transformation|GetActorLocation) "0, 0, 0" 1.0 1.0 0.0 "/Game/FPSAssets/Sounds/Attunation/CasingAttunation.CasingAttunation" 0 0 0)
        (bind (_outactors _returnvalue) (Collision|SphereOverlapActors (Transformation|GetWorldLocation (Variables|Default|GetArrow1)) 8e+01 (Utilities|Array|MakeArray "ObjectTypeQuery3") "/Game/FPSAssets/FirstPersonBP/Blueprints/FirstPersonCharacter.FirstPersonCharacter_C" (Utilities|Array|MakeArray self)))
        (if _returnvalue
          (for _array_element _outactors
            (Game|Damage|ApplyDamage _array_element 2e+01 (Game|GetInstigatorController) self "/Script/Engine.DamageType")))))))

(event Custom|Death
  ;[1 1 1] death logic
  (Variables|Default|SetIsDead true)
  (Components|Movement|StopMovementImmediately (Variables|Character|GetCharacterMovement))
  (Animation|Montage|PlayMontage (Variables|Character|GetMesh) "/Game/FPSAssets/Zombie/Animations/zombie_dying_Montage.zombie_dying_Montage"))

(event EventBeginPlay
  (CallFunction|MovetoPlayer))

(event Game|Damage|EventPointDamage
  (params (Damage :type Float%20%28single-precision%29) (DamageType :type Damage%20Type%20Object%20Reference) (HitLocation :type Vector :default "0, 0, 0") (HitNormal :type Vector :default "0, 0, 0") (HitComponent :type Primitive%20Component%20Object%20Reference) (BoneName :type Name :default "None") (ShotFromDirection :type Vector :default "0, 0, 0") (InstigatedBy :type Controller%20Object%20Reference) (DamageCauser :type Actor%20Object%20Reference) (HitInfo :type Hit%20Result%20Structure%20%28by%20ref%29))
  ;[1 1 1] damage logic
  (if (not (Variables|Default|GetIsDead))
    (if (<= (Variables|Default|GetHealth) Damage)
      (CallFunction|Death)
      (Collision|SetCollisionResponsetoChannel (Variables|Collision|GetCapsuleComponent) "ECC_Pawn" "ECR_Overlap")
      (Collision|SetCollisionEnabled (Variables|Character|GetMesh) "NoCollision")
      (bind _asbp_zombie_game_mode (Utilities|Casting|CastToBP_ZombieGameMode (Game|GetGameMode)))
      (Default|ZombieKilled _asbp_zombie_game_mode)
      (Utilities|FlowControl|Delay 5.0)
      (Actor|DestroyActor)
      (else
        (Variables|Default|SetHealth (- (Variables|Default|GetHealth) Damage))
        (Animation|Montage|PlayMontage (Variables|Character|GetMesh) "/Game/FPSAssets/Zombie/Animations/Zombie_Reaction_Hit_mixamo_com_Montage.Zombie_Reaction_Hit_mixamo_com_Montage")))))

(fn ConstructionScript)